(event Custom|Reset%20Game
  ;[1 1 1] Reset the points and turn off "You win" message
  (Variables|Default|SetcurrentPoints 0)
  (Variables|/Game/Blueprints/BP_GameUI.BP_GameUI_C|Setpoint (Variables|Default|GetcurrentUI) 0))

(event Custom|Update%20Points
  ;[1 1 1] Increment point and update UI
  (bind _output_get (Variables|Default|SetcurrentPoints (+ 1 (Variables|Default|GetcurrentPoints))))
  (Variables|/Game/Blueprints/BP_GameUI.BP_GameUI_C|Setpoint (Variables|Default|GetcurrentUI) _output_get)
  (CallFunction|EndGame))

(event Custom|End%20Game
  ;[1 1 1] Check to see if all pickups collected
  (if (>= (Variables|Default|GetcurrentPoints) (Variables|Default|GetcountPickUps))
    (Variables|/Game/Blueprints/BP_GameUI.BP_GameUI_C|SetyouWinOpacity (Variables|Default|GetcurrentUI) 1.0)))

(event EventBeginPlay
  ;[1 1 1] Create a new instance of a UI and add it to screen
  (Utilities|FlowControl|Sequence
    (:then_0
      (bind _returnvalue (UserInterface|CreateWidget "/Game/Blueprints/BP_GameUI.BP_GameUI_C"))
      (bind _output_get (Variables|Default|SetcurrentUI _returnvalue))
      (UserInterface|Viewport|AddtoViewport _output_get 0))
    (:then_1
      (bind _outactors (Actor|GetAllActorsOfClass "/Game/Blueprints/BP_PickUps.BP_PickUps_C"))
      (Variables|Default|SetcountPickUps (Utilities|Array|Length _outactors))))
  (CallFunction|ResetGame))

(fn ConstructionScript)